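; BP_MainGameMode is the main game mode that tracks the stage countdown timer and the score.
; BeginPlay sets the stage time to its maximum, and Tick counts it down until it would drop below zero, then sets the time-limit flag.
; Functions reset the timer and flag, add to the score, and expose the time, score and time-limit state to other Blueprints.
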(event EventBeginPlay
  (Variables|Default|SetStageTime (Variables|Default|GetMaxStageTime) :!pinned true) ; ステージタイムをMaxTimeと同じ値にする
)

(event EventTick
  (params (DeltaSeconds :type Float%20%28single-precision%29))
  (if (< (- (Variables|Default|GetStageTime) DeltaSeconds) 0.0)
    (Variables|Default|SetisTimeLimit? true) ; タイムリミット！
    (else
      (Variables|Default|SetStageTime (- (Variables|Default|GetStageTime) DeltaSeconds) :!pinned true) ; ステージのタイムを更新する
    )))

(fn ConstructionScript)

(fn FResetTime
  (Variables|Default|SetStageTime (Variables|Default|GetMaxStageTime))
  (Variables|Default|SetisTimeLimit? false)
  (return))

(fn FAddScore
  (params (AddScore :type Integer))
  (Variables|Default|SetScore (+ (Variables|Default|GetScore) AddScore))
  (return))

(fn FGetTimeLimit
  (return (Variables|Default|GetisTimeLimit?)))

(fn FGetScore
  (return (Variables|Default|GetScore)))

(fn FGetStageTime
  (return (Variables|Default|GetStageTime)))