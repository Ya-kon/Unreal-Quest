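; BP_Enemy is an enemy pawn that chases the player on sight and kills them on contact.
; PawnSensing's See Pawn event issues AIMoveTo toward player 0, then immediately stops active movement if the player is over 1000 units away.
; Overlapping SphereAttackCollision with a ThirdPersonCharacter calls that character's FPhysicsOnDead.
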(event OnComponentBeginOverlap(Sphere＿AttackCollision)
  (params (OverlappedComponent :type Primitive%20Component%20Object%20Reference) (OtherActor :type Actor%20Object%20Reference) (OtherComp :type Primitive%20Component%20Object%20Reference) (OtherBodyIndex :type Integer) (bFromSweep :type Boolean) (SweepResult :type Hit%20Result%20Structure%20%28by%20ref%29))
  (bind _asthird_person_character (Utilities|Casting|CastToThirdPersonCharacter OtherActor))
  (Default|FPhysicsonDead _asthird_person_character :!pinned true) ; プレイヤーを死亡させる
)

(event OnSeePawn(PawnSensing)
  (params (Pawn :type Pawn%20Object%20Reference))
  (AI|AIMoveTo self "0, 0, 0" (Game|GetPlayerCharacter 0) 5.0 false ; プレイヤーを追いかける
    (:then
      (if (> (Math|Vector|Distance(Vector) (Transformation|GetActorLocation) (Transformation|GetActorLocation (Game|GetPlayerCharacter 0))) 1e+03)
        (Class|NavMovementComponent|StopActiveMovement (Variables|Character|GetCharacterMovement) :!pinned true) ; Movementの移動を止める
      ))))

(fn ConstructionScript)