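; BP_MoveFloor is a moving-floor gimmick actor that travels along one world axis.
; BeginPlay passes MoveDirection to the EMoveFloor event, which starts the TL_Move timeline from the beginning.
; Each timeline update switches on the direction to pick X, Y or Z and adds MoveValue to the current location.
; The curve therefore acts as a per-update step that accumulates, rather than an offset from the start position.
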(event Custom|E_MoveFloor
  (params (MoveDirection :type Integer))
  (bind _returnvalue (Transformation|GetActorLocation))
  (bind _returnvalue_2 (Transformation|GetActorLocation))
  (bind _returnvalue_3 (Transformation|GetActorLocation))
  ;[1 1 1] E_MoveFloor
  (bind _movevalue (Timeline|TL_Move PlayFromStart) ; 移動量をタイムラインで制御する
    (:Update
      (switch int MoveDirection ; MoveDirectionの値から分岐する
        (:0
          ;;[1 1 1] Xの+方向に動かす
          (Transformation|SetActorLocation (Math|Vector|MakeVector (+ _movevalue (.x _returnvalue_2)) (.y _returnvalue_2) (.z _returnvalue_2)) false false))
        (:1
          ;;[1 1 1] Yの+方向に動かす
          (Transformation|SetActorLocation (Math|Vector|MakeVector (.x _returnvalue_3) (+ _movevalue (.y _returnvalue_3)) (.z _returnvalue_3)) false false))
        (:2
          ;;[1 1 1] Zの+方向に動かす
          (Transformation|SetActorLocation (Math|Vector|MakeVector (.x _returnvalue) (.y _returnvalue) (+ _movevalue (.z _returnvalue))) false false))))))

(event EventBeginPlay
  ;[1 1 1] Begin Play
  (CallFunction|EMoveFloor (Variables|Default|GetMoveDirection) :!pinned true) ; 床を動かす\n指定した方向の＋の向きに動かす
)

(fn ConstructionScript)