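; BP_FallFloor is a gimmick floor that disappears after the player steps into its trigger and later comes back.
; An overlap on Box_Collision by an actor tagged "Player" turns SMFloor red as a warning, then after a delay hides it and disables its collision.
; A second delay restores visibility, query-only collision and the green material, all sequenced with latent Delays in the event graph.
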(event OnComponentBeginOverlap(Box_Collision)
  (params (OverlappedComponent :type Primitive%20Component%20Object%20Reference) (OtherActor :type Actor%20Object%20Reference) (OtherComp :type Primitive%20Component%20Object%20Reference) (OtherBodyIndex :type Integer) (bFromSweep :type Boolean) (SweepResult :type Hit%20Result%20Structure%20%28by%20ref%29))
  (bind _sm_floor (Variables|Default|GetSM_Floor))
  (bind _sm_floor_2 (Variables|Default|GetSM_Floor))
  (if (Actor|ActorHasTag OtherActor "Player")
    (Rendering|Material|SetMaterial (Variables|Default|GetSM_Floor) 0 "/Game/00_WorkSpace/Material/MI_BaseColor_Red.MI_BaseColor_Red" :!pinned true) ; Floorのマテリアルを変更
    (Utilities|FlowControl|Delay 3.0) ; 処理を遅らせる
    (Rendering|SetVisibility _sm_floor_2 false false :!pinned true) ; Floorを見た目を非表示にする
    (Collision|SetCollisionEnabled _sm_floor_2 "NoCollision" :!pinned true) ; Floorのコリジョン判定を消す
    (Utilities|FlowControl|Delay 4.0) ; 処理を遅らせる
    ;[1 1 1] 元に戻す
    (Rendering|SetVisibility _sm_floor true false)
    (Collision|SetCollisionEnabled _sm_floor "QueryOnly")
    (Rendering|Material|SetMaterial _sm_floor 0 "/Game/00_WorkSpace/Material/MI_Green.MI_Green")))

(fn ConstructionScript)